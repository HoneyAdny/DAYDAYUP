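; Dissolve demo actor with two character meshes, Gwen and GwenBlack, that share one DissolveValue, with RevertDissolve enabled only on GwenBlack.
; The construction script pushes both parameters to the mesh materials and DissolveValue to a dynamic instance of GwenBlack's overlay material.
; BeginPlay wraps that overlay in another dynamic instance.
; The Timeline that would animate the dissolve is unconnected, so nothing changes the value at runtime.
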(event `self.ReceiveBeginPlay`
  (bind _gwen_black (`self.Gwen_black`))
  (bind _returnvalue (`KismetMaterialLibrary.CreateDynamicMaterialInstance` (`MeshComponent.OverlayMaterial` _gwen_black) "None" "Transient"))
  (`MeshComponent.SetOverlayMaterial` _gwen_black _returnvalue))

(event `self.ReceiveTick`
  (params (DeltaSeconds :type "Float (single-precision)")))

(fn `UserConstructionScript`
  (bind _gwen_black (`self.Gwen_black`))
  (bind _dissolvevalue (`self.DissolveValue`))
  (bind _gwen_black_2 (`self.Gwen_black`))
  (`MeshComponent.SetScalarParameterValueOnMaterials` _gwen_black "RevertDissolve" 1.0)
  (`MeshComponent.SetScalarParameterValueOnMaterials` (`self.Gwen`) "RevertDissolve" 0.0)
  (`MeshComponent.SetScalarParameterValueOnMaterials` _gwen_black "DissolveValue" _dissolvevalue)
  (`MeshComponent.SetScalarParameterValueOnMaterials` (`self.Gwen`) "DissolveValue" _dissolvevalue)
  (bind _returnvalue (`KismetMaterialLibrary.CreateDynamicMaterialInstance` (`MeshComponent.OverlayMaterial` _gwen_black_2) "None" "Transient"))
  (`MeshComponent.SetOverlayMaterial` _gwen_black_2 _returnvalue)
  (`MaterialInstanceDynamic.SetScalarParameterValue` _returnvalue "DissolveValue" _dissolvevalue))