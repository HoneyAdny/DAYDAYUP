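; BP_Gwen is a dissolve demo actor with two mesh components, Gwen and GwenBlack, driven by a shared material dissolve effect.
; The construction script sets RevertDissolve to opposite values on the two meshes and applies the DissoveValue variable to both.
; Two seconds after BeginPlay, a Timeline animates DissolveValue on both meshes together.
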(event `self.ReceiveTick`
  (params (DeltaSeconds :type "Float (single-precision)")))

(event `self.ReceiveBeginPlay`
  (`KismetSystemLibrary.Delay` 2.0)
  (bind (_direction _newtrack_0) (`Timeline|Timeline`)
    (:`Update`
      (`MeshComponent.SetScalarParameterValueOnMaterials` (`self.Gwen_Black`) "DissolveValue" _newtrack_0)
      (`MeshComponent.SetScalarParameterValueOnMaterials` (`self.Gwen`) "DissolveValue" _newtrack_0))))

(fn `UserConstructionScript`
  (bind _gwen (`self.Gwen`))
  (`MeshComponent.SetScalarParameterValueOnMaterials` (`self.Gwen_Black`) "RevertDissolve" 1.0)
  (`MeshComponent.SetScalarParameterValueOnMaterials` _gwen "RevertDissolve" 0.0)
  (`MeshComponent.SetScalarParameterValueOnMaterials` _gwen "DissolveValue" (`self.DissoveValue`))
  (`MeshComponent.SetScalarParameterValueOnMaterials` (`self.Gwen_Black`) "DissolveValue" (`self.DissoveValue`)))