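; Dissolve demo Blueprint that animates a dissolve effect by driving parameters in the MPC_Dissolve2_kz material parameter collection.
; On BeginPlay, four timelines start together and write the WPO, noise, Color and mask parameters on each update.
; A separate mask event plays another timeline that, despite the event's name, also writes WPO; nothing in this graph calls it.
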(event `mask`
  (bind (_direction _1) (`Timeline|Timeline` :!via `PlayFromStart`)
    (:`Update`
      (`KismetMaterialLibrary.SetScalarParameterValue` "/Game/DissolveDemo/Dissolve2/MPC_Dissolve2_kz.MPC_Dissolve2_kz" "WPO" _1))))

(event `self.ReceiveBeginPlay`
  (`|ExecutionSequence`
    (:`then_0`
      (bind (_direction _1) (`Timeline|Timeline_wpo` :!via `PlayFromStart`)
        (:`Update`
          (`KismetMaterialLibrary.SetScalarParameterValue` "/Game/DissolveDemo/Dissolve2/MPC_Dissolve2_kz.MPC_Dissolve2_kz" "WPO" _1))))
    (:`then_1`
      (bind (_direction_2 _2) (`Timeline|Timeline_noise` :!via `PlayFromStart`)
        (:`Update`
          (`KismetMaterialLibrary.SetScalarParameterValue` "/Game/DissolveDemo/Dissolve2/MPC_Dissolve2_kz.MPC_Dissolve2_kz" "noise" _2))))
    (:`then_2`
      (bind (_direction_3 _2_2) (`Timeline|Timeline_cloor` :!via `PlayFromStart`)
        (:`Update`
          (`KismetMaterialLibrary.SetVectorParameterValue` "/Game/DissolveDemo/Dissolve2/MPC_Dissolve2_kz.MPC_Dissolve2_kz" "Color" (`KismetMathLibrary.Conv_DoubleToLinearColor` _2_2)))))
    (:`then_3`
      (bind (_direction_4 _1_2) (`Timeline|Timeline_mask` :!via `PlayFromStart`)
        (:`Update`
          (`KismetMaterialLibrary.SetScalarParameterValue` "/Game/DissolveDemo/Dissolve2/MPC_Dissolve2_kz.MPC_Dissolve2_kz" "mask" _1_2))))))

(fn `UserConstructionScript`)