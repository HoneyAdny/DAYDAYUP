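; Bottle actor that fakes wobbling liquid in its mesh by driving a dynamic material instance created on BeginPlay.
; Each tick, a clamped, underdamped vector spring trails the actor's location.
; The spring's vertical lag becomes LiquidHeight and its horizontal lag tilts the up vector into LiquidDir, both sent to the material.
; A debug arrow and print remain active, while an older height-only float spring is left unconnected.
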(event `self.ReceiveBeginPlay`
  (bind _returnvalue (`KismetMaterialLibrary.CreateDynamicMaterialInstance` (`self.ParentMaterial`) "waterHeight"))
  (bind _output_get (set `self.Current Materila` _returnvalue))
  (`PrimitiveComponent.SetMaterial` (`self.MilkBottle`) 0 _output_get))

(event `self.ReceiveTick`
  (params (DeltaSeconds :type "Float (single-precision)"))
  (bind _current_materila (`self.Current Materila`))
  (bind (_liquidheight _liquedir) (`self.CaleLiquidSurface`))
  (`MaterialInstanceDynamic.SetScalarParameterValue` _current_materila "LiquidHeight" _liquidheight)
  (`MaterialInstanceDynamic.SetVectorParameterValue` _current_materila "LiquidDir" (`KismetMathLibrary.Conv_VectorToLinearColor` _liquedir))
  (`KismetSystemLibrary.PrintString` (`KismetStringLibrary.Conv_VectorToString` _liquedir)))

(fn `CaleLiquidSurface`
  (returns (LiquidHeight :type "Float (double-precision)") (LiqueDir :type "Vector Structure") (NewParam :type "Vector Structure"))
  (bind _returnvalue (`self.K2_GetActorLocation`))
  (bind _liquidlocationoffset (`self.LiquidLocationOffset`))
  (bind (_returnvalue_x _returnvalue_y) (`KismetMathLibrary.BreakVector` (- (`self.SpringLiquidLocation`) (`self.K2_GetActorLocation`))))
  (bind _returnvalue_2 (`KismetMathLibrary.MakeVector` _returnvalue_x _returnvalue_y))
  (bind _returnvalue_3 (`KismetMathLibrary.VectorSpringInterp` (`self.SpringLiquidLocation`) _returnvalue (`self.SpringStateLiquidHeight vector`) 150.0 0.2 (`GameplayStatics.GetWorldDeltaSeconds`) 1.0 0.2 true (- _returnvalue _liquidlocationoffset) (+ _returnvalue _liquidlocationoffset) true))
  (bind _output_get (set `self.SpringLiquidLocation` _returnvalue_3))
  (`KismetSystemLibrary.DrawDebugArrow` (`self.K2_GetActorLocation`) (`self.SpringLiquidLocation`) 1.0 (struct :`R` 1.0 :`G` 0.629519 :`B` 0.020388 :`A` 1.0) 0.0 0.2)
  (return (- (.z _output_get) (.z (`self.K2_GetActorLocation`))) (`KismetMathLibrary.Vector_SlerpVectorToDirection` (0.0 0.0 1.0) _returnvalue_2 (`KismetMathLibrary.VSize` _returnvalue_2)) (0.0 0.0 0.0)))

(fn `UserConstructionScript`)