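; BP_Velet is an actor that visualizes two vector parameters from a Material Parameter Collection as the world positions of its Red and Green components.
; Every Tick it reads LDitr and OtherVector, scales them by 100 and moves Red and Green to those locations.
; Disconnected nodes hold an unfinished write-back of Red's location to the collection and a construction-script copy of the same logic.
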(event `self.ReceiveTick`
  (params (DeltaSeconds :type "Float (single-precision)"))
  (bind _returnvalue (`KismetMaterialLibrary.GetVectorParameterValue` (`self.MPC`) (`self.LDitr`)))
  (bind _returnvalue_2 (`KismetMaterialLibrary.GetVectorParameterValue` (`self.MPC`) (`self.Other Vector`)))
  (`SceneComponent.K2_SetWorldLocation` (`self.Red`) (* (`KismetMathLibrary.Conv_LinearColorToVector` _returnvalue) (100.0 100.0 100.0)) false false)
  (`SceneComponent.K2_SetWorldLocation` (`self.Green`) (* (`KismetMathLibrary.Conv_LinearColorToVector` _returnvalue_2) (100.0 100.0 100.0)) false false))

(fn `UserConstructionScript`)