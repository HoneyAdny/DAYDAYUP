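; Geometry Script generated mesh actor that prototypes snow placement on a chosen actor's mesh.
; On rebuild, it copies that actor's root component mesh into a compute mesh, builds a BVH and copies the mesh to the output.
; A short loop casts downward rays from seeded random XY points within the bounds, starting at bounding-box height plus an offset.
; Each hit appends a sphere-box primitive to the output as a snow blob.
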(event `self.OnRebuildGeneratedMesh`
  (params (TargetMesh :type "DynamicMesh Object Reference"))
  (bind _stream (`self.Stream`))
  (set `self.Target Mesh` TargetMesh)
  (`|ExecutionSequence`
    (:`then_0`
      (bind _returnvalue (`self.AllocateComputeMesh`))
      (set `self.RaycastMeshActors` _returnvalue)
      (bind __meshtoaddsnowtoo (`self. MeshToAddSnowToo`)
        (:`then`
          (`GeometryScriptLibrary_SceneUtilityFunctions.CopyMeshFromComponent` (`Actor.RootComponent` __meshtoaddsnowtoo) (`self.RaycastMeshActors`) (struct) false null))
        (:`else`)))
    (:`then_1`
      (bind (_outputbvh _returnvalue_2) (`GeometryScriptLibrary_MeshSpatial.BuildBVHForMesh` (`self.RaycastMeshActors`) null))
      (set `self.Output BVH` _outputbvh)
      (`GeometryScriptLibrary_MeshDecompositionFunctions.CopyMeshToMesh` (`self.RaycastMeshActors`) (`self.Target Mesh`) null)
      (for _ (range 17)
        (bind _returnvalue_3 (`GeometryScriptLibrary_MeshQueryFunctions.GetMeshBoundingBox` _returnvalue_2))
        (bind _hitresult (`GeometryScriptLibrary_MeshSpatial.FindNearestRayIntersectionWithMesh` (`self.RaycastMeshActors`) (`self.Output BVH`) (`KismetMathLibrary.MakeVector` (`KismetMathLibrary.RandomFloatInRangeFromStream` _stream (.x (break `Box` _returnvalue_3)) (.x (`.Max` (break `Box` _returnvalue_3)))) (`KismetMathLibrary.RandomFloatInRangeFromStream` _stream (.y (break `Box` _returnvalue_3)) (.y (`.Max` (break `Box` _returnvalue_3)))) (+ (- (.z (`.Max` (break `Box` _returnvalue_3))) (.z (break `Box` _returnvalue_3))) 50.0)) (0.0 0.0 -1.0) (struct) null)
          (:`Found`
            (`GeometryScriptLibrary_MeshPrimitiveFunctions.AppendSphereBox` (`self.Target Mesh`) (struct) (`KismetMathLibrary.MakeTransform` (`.HitPosition` (break `GeometryScriptRayHitResult` _hitresult))) 50.0 6 6 6 "Center" null)))))))

(fn `UserConstructionScript`)